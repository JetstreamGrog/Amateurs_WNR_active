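; Clock Blueprint that animates its second, minute and hour hands by stepping their relative roll.
; Tick drives three chained Delays, each followed by a fixed roll increment on one hand, with no reading of actual time.
; Delays ignore re-triggers while pending, so seconds step about every second and minutes about every minute.
; The hour hand follows each minute step 59 seconds later, so it advances a full hour mark roughly every minute.
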(event `self.ReceiveTick`
  (params (DeltaSeconds :type "Float (single-precision)"))
  (bind _secondes_clock (`self.Secondes_Clock`))
  (bind _minutes_clock (`self.Minutes_Clock`))
  (bind _hours_clock (`self.Hours_Clock`))
  (bind (_relativerotation_roll _relativerotation_pitch _relativerotation_yaw) (`KismetMathLibrary.BreakRotator` (`SceneComponent.RelativeRotation` _hours_clock)))
  (bind (_relativerotation_roll_2 _relativerotation_pitch_2 _relativerotation_yaw_2) (`KismetMathLibrary.BreakRotator` (`SceneComponent.RelativeRotation` _secondes_clock)))
  (bind (_relativerotation_roll_3 _relativerotation_pitch_3 _relativerotation_yaw_3) (`KismetMathLibrary.BreakRotator` (`SceneComponent.RelativeRotation` _minutes_clock)))
  (`KismetSystemLibrary.Delay` 1.0)
  (`SceneComponent.K2_SetRelativeRotation` _secondes_clock (`KismetMathLibrary.MakeRotator` (+ _relativerotation_roll_2 6.0) _relativerotation_pitch_2 _relativerotation_yaw_2) false false)
  (`KismetSystemLibrary.Delay` 60.0)
  (`SceneComponent.K2_SetRelativeRotation` _minutes_clock (`KismetMathLibrary.MakeRotator` (+ _relativerotation_roll_3 6.0) _relativerotation_pitch_3 _relativerotation_yaw_3) false false)
  (`KismetSystemLibrary.Delay` 59.0)
  (`SceneComponent.K2_SetRelativeRotation` _hours_clock (`KismetMathLibrary.MakeRotator` (+ _relativerotation_roll 30.0) _relativerotation_pitch _relativerotation_yaw) false false))

(fn `UserConstructionScript`)