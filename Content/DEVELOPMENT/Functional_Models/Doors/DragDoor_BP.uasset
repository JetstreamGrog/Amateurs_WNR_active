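; Draggable door actor that the player swings by holding the DragDoor input and turning.
; On press, it line-traces from the CharacterJack_BP camera against WorldDynamic objects and flags a hit on any DragDoor_BP, without checking for this instance.
; While held and flagged, Tick adds the character's TurnRate, scaled by Sensitivity, to the door's yaw, clamped between angle limits.
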(event `self.ReceiveTick`
  (params (DeltaSeconds :type "Float (single-precision)"))
  (bind (_relativerotation_roll _relativerotation_pitch _relativerotation_yaw) (`KismetMathLibrary.BreakRotator` (`SceneComponent.RelativeRotation` (`self.Door`))))
  (if (`self.IsHoldingLMB?`)
    (if (`self.IsLookingAtDoor?`)
      (if true
        (`SceneComponent.K2_SetRelativeRotation` (`self.Door`) (`KismetMathLibrary.MakeRotator` 0.0 0.0 (`KismetMathLibrary.FClamp` (+ (* (`/Game/DEVELOPMENT/Beta_Character/CharacterJack_BP.Turn Rate` (stale `InputAction|DragDoor` _ascharacter_jack_bp)) (`self.Sensitivity`)) _relativerotation_yaw) (`self.Min Angle`) (`self.Max Angle`))) false false)))))

(event `self.ReceiveBeginPlay`
  (`self.EnableInput` (`GameplayStatics.GetPlayerController` 0))
  (`self.SetOwner` null))

(event `InputAction|DragDoor`
  (params (Key :type "Key Structure"))
  ;[1 1 1] Check if is looking at the door
  (:`Pressed`
    (set `self.IsHoldingLMB?` true)
    (bind _ascharacter_jack_bp (cast `/Game/DEVELOPMENT/Beta_Character/CharacterJack_BP` (`GameplayStatics.GetPlayerCharacter` 0)))
    (bind _camerajack (`/Game/DEVELOPMENT/Beta_Character/CharacterJack_BP.CameraJack` _ascharacter_jack_bp))
    (bind _returnvalue (`SceneComponent.K2_GetComponentLocation` _camerajack))
    (bind (_outhit _returnvalue_2) (`KismetSystemLibrary.LineTraceSingleForObjects` :`Start` _returnvalue :`End` (+ _returnvalue (* (`SceneComponent.GetForwardVector` _camerajack) 500.0)) :`ObjectTypes` (`|MakeArray` "ObjectTypeQuery2" :!type "EObjectTypeQuery Enum") :`bIgnoreSelf` false))
    (if _returnvalue_2
      (cast `/Game/DEVELOPMENT/Functional_Models/Doors/DragDoor_BP` (`.HitActor` (`GameplayStatics.BreakHitResult` _outhit)))
      (set `self.IsLookingAtDoor?` true)
      (else
        (set `self.IsLookingAtDoor?` false))))
  (:`Released`
    (set `self.IsHoldingLMB?` false)))

(fn `Check Location Acc to Mesh`
  (params (Actor :type "ActorLayer Structure")))

(fn `UserConstructionScript`)