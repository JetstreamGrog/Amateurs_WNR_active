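; Character Blueprint that handles basic player movement and camera look from axis inputs.
; Forward and strafe inputs move the character relative to the control rotation's yaw only, ignoring pitch and roll.
; Look inputs are clamped to a -1 to 1 range before feeding controller pitch and yaw.
; The construction script is empty.
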(event `InputAxis|Forwards/Backward`
  (params (AxisValue :type "Float (single-precision)"))
  (`self.AddMovementInput` (`KismetMathLibrary.GetForwardVector` (`KismetMathLibrary.MakeRotator` 0.0 0.0 (.yaw (`self.GetControlRotation`)))) AxisValue))

(event `InputAxis|Right/Left`
  (params (AxisValue :type "Float (single-precision)"))
  (`self.AddMovementInput` (`KismetMathLibrary.GetRightVector` (`KismetMathLibrary.MakeRotator` 0.0 0.0 (.yaw (`self.GetControlRotation`)))) AxisValue))

(event `InputAxis|LookUP/LookDown`
  (params (AxisValue :type "Float (single-precision)"))
  (`self.AddControllerPitchInput` (`KismetMathLibrary.FClamp` AxisValue -1.0)))

(event `InputAxis|LookRight/LookLeft`
  (params (AxisValue :type "Float (single-precision)"))
  (`self.AddControllerYawInput` (`KismetMathLibrary.FClamp` AxisValue -1.0)))

(fn `UserConstructionScript`)